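; BP_Door is a double sliding door that opens automatically at BeginPlay.
; BeginPlay caches both panels' relative start locations, then calls OpenDoor, which slides them apart along local X by DoorMaxRange using a timeline-driven lerp.
; CloseDoor lerps them back on a separate timeline but is not called within this Blueprint.
; Both timelines use Play rather than PlayFromStart, so neither restarts once finished.
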(event Custom|OpenDoor
  (bind _leftdoorinitlocation (Variables|Default|GetLeftDoorInitLocation))
  (bind _rightdoorinitlocation (Variables|Default|GetRightDoorInitLocation))
  ;[0.15 0.15 0.15 0.5] Open Door
  (bind _newtrack_0 (Timeline|Timeline Play)
    (:Update
      (Transformation|SetRelativeLocation (Variables|Default|GetRightDoor) (Math|Vector|Lerp(Vector) _rightdoorinitlocation (+ _rightdoorinitlocation (Math|Vector|MakeVector (Variables|Default|GetDoorMaxRange) 0.0 0.0)) _newtrack_0) false false)
      (Transformation|SetRelativeLocation (Variables|Default|GetLeftDoor) (Math|Vector|Lerp(Vector) _leftdoorinitlocation (- _leftdoorinitlocation (Math|Vector|MakeVector (Variables|Default|GetDoorMaxRange) 0.0 0.0)) _newtrack_0) false false))))

(event Custom|CloseDoor
  (bind _rightdoorinitlocation (Variables|Default|GetRightDoorInitLocation))
  (bind _doormaxrange (Variables|Default|GetDoorMaxRange))
  (bind _leftdoorinitlocation (Variables|Default|GetLeftDoorInitLocation))
  (bind _doormaxrange_2 (Variables|Default|GetDoorMaxRange))
  (bind _returnvalue (- _leftdoorinitlocation (Math|Vector|MakeVector _doormaxrange_2 0.0 0.0)))
  (bind _returnvalue_2 (+ _rightdoorinitlocation (Math|Vector|MakeVector _doormaxrange 0.0 0.0)))
  ;[0.15 0.15 0.15 0.5] Close Door
  (bind _newtrack_0 (Timeline|Timeline_0 Play)
    (:Update
      (Transformation|SetRelativeLocation (Variables|Default|GetRightDoor) (Math|Vector|Lerp(Vector) _returnvalue_2 (- _returnvalue_2 (Math|Vector|MakeVector (Variables|Default|GetDoorMaxRange) 0.0 0.0)) _newtrack_0) false false)
      (Transformation|SetRelativeLocation (Variables|Default|GetLeftDoor) (Math|Vector|Lerp(Vector) _returnvalue (+ _returnvalue (Math|Vector|MakeVector (Variables|Default|GetDoorMaxRange) 0.0 0.0)) _newtrack_0) false false))))

(event EventBeginPlay
  (Variables|Default|SetRightDoorInitLocation (Variables|/Script/Engine.SceneComponent|GetRelativeLocation (Variables|Default|GetRightDoor)))
  (Variables|Default|SetLeftDoorInitLocation (Variables|/Script/Engine.SceneComponent|GetRelativeLocation (Variables|Default|GetLeftDoor)))
  (CallFunction|OpenDoor))

(event Collision|EventActorBeginOverlap
  (params (OtherActor :type Actor%20Object%20Reference)))

(event EventTick
  (params (DeltaSeconds :type Float%20%28single-precision%29)))

(fn ConstructionScript)